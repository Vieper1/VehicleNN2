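; Walled road generator Blueprint that lays groundwork for building a track along a spline, still at an early stage.
; The Construction Script stores the spline point count and grows or trims RoadDataArray until it holds one entry per point.
; BuildTrackElement so far only computes a segment's current and wrapped next point index, and nothing shown calls it or creates meshes.
; The event graph holds only disabled stub events.
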(event EventBeginPlay)

(event Collision|EventActorBeginOverlap
  (params (OtherActor :type Actor%20Object%20Reference)))

(event EventTick
  (params (DeltaSeconds :type Float%20%28single-precision%29)))

(fn ConstructionScript
  (bind _roaddataarray (Variables|Default|GetRoadDataArray))
  (Utilities|FlowControl|Sequence
    (:then_0
      ;[1 1 1] Store number of spline points
      (Variables|Default|SetnumberOfSplinePoints (Spline|GetNumberOfSplinePoints (Variables|Default|GetSpline))))
    (:then_1
      ;[1 1 1] Build RoadArray data
      (Math|Integer|CompareInt (Utilities|Array|Length (Variables|Default|GetRoadDataArray)) (Variables|Default|GetnumberOfSplinePoints) :!label _label
        (:>
          (Utilities|Array|RemoveIndex _roaddataarray (Utilities|Array|LastIndex _roaddataarray))
          (goto _label))
        (:<
          (Utilities|Array|Add :TargetArray _roaddataarray)
          (goto _label))))
    (:then_2)
    (:then_3)))

(fn BuildTrackElement
  (params (LoopIndex :type Integer))
  (LocalVariables|SetLocalLoopIndex LoopIndex)
  (LocalVariables|SetLocalNextLoopIndex (Math|Integer|%(Integer) (+ LoopIndex 1) (Variables|Default|GetnumberOfSplinePoints))))