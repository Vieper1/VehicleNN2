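; ColliderBP is a vehicle-project actor that reports a 0 to 1 activation value derived from a spring arm, apparently serving as a distance sensor.
; Each Tick it divides the distance between SphereIndicator and SpringArm by the arm's TargetArmLength and clamps the result into ColliderActivation.
; GetActivationValue exposes that value, which reads 1 at full arm length and falls as the indicator nears the arm's origin.
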(event EventBeginPlay)

(event Collision|EventActorBeginOverlap
  (params (OtherActor :type Actor%20Object%20Reference)))

(event EventTick
  (params (DeltaSeconds :type Float%20%28single-precision%29))
  (bind _springarm (Variables|Default|GetSpringArm))
  (bind _sphereindicator (Variables|Default|GetSphereIndicator))
  (bind _returnvalue (Transformation|GetWorldLocation _sphereindicator))
  (bind _returnvalue_2 (Transformation|GetWorldLocation _springarm))
  (bind _targetarmlength (Variables|/Script/Engine.SpringArmComponent|GetTargetArmLength _springarm))
  (bind _returnvalue_3 (- _returnvalue _returnvalue_2))
  (bind _returnvalue_4 (Math|Vector|VectorLength _returnvalue_3))
  (bind _returnvalue_5 (/ _returnvalue_4 _targetarmlength))
  (if (< _returnvalue_5 0.0)
    (Variables|Default|Setcollider_activation 0.0)
    (elif (> _returnvalue_5 1.0)
      (Variables|Default|Setcollider_activation 1.0)
      (else
        (Variables|Default|Setcollider_activation _returnvalue_5)))))

(fn ConstructionScript)

(fn GetActivationValue
  (return (Variables|Default|Getcollider_activation)))